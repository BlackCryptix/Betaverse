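; Player controller that manages the HUD, pause menu, text chat and interaction with 3D world widgets.
; A WidgetInteraction component relays clicks and keys, and reports hover changes to the HUD.
; Entering 3D widget mode switches the pointer from screen center to mouse, focuses the widget and disables pawn input until game mode is restored.
; The pause menu is created lazily and toggled, switching input modes and cursor visibility.
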(event `Key|LeftMouseButton`
  (params (Key :type "Key Structure"))
  (bind _widgetinteractioncomp (`self.WidgetInteractionComp`))
  (:`Pressed`
    (`WidgetInteractionComponent.PressPointerKey` _widgetinteractioncomp "LeftMouseButton"))
  (:`Released`
    (`WidgetInteractionComponent.ReleasePointerKey` _widgetinteractioncomp "LeftMouseButton")
    (bind _focusewidget (`self.FocuseWidget`)
      (:`then`
        (`Widget.SetKeyboardFocus` _focusewidget))
      (:`else`))))

(event `self.ReceiveBeginPlay`
  (if (`self.IsLocalController`)
    (`WidgetBlueprintLibrary.SetInputMode_GameOnly` self)
    (set `self.bShowMouseCursor` false)
    (bind _returnvalue (`|CreateWidget` "/Game/PlayerCharacter/Hud/W_Hud.W_Hud_C" self))
    (bind _output_get (set `self.Hud` _returnvalue))
    (`UserWidget.AddToViewport` _output_get 0)
    (add `WidgetInteractionComponent.OnHoveredWidgetChanged` (`self.WidgetInteractionComp`) (delegate `OnHoveredWidgetChanged_Event_0`))))

(event `OnHoveredWidgetChanged_Event_0`
  (params (WidgetComponent :type "WidgetComponent Object Reference") (PreviousWidgetComponent :type "WidgetComponent Object Reference"))
  (`/Game/PlayerCharacter/Hud/W_Hud.OnCanInteractChanged_Event_0` (`self.Hud`) (`KismetSystemLibrary.IsValid` WidgetComponent)))

(event `KeyboardKeyPressedWithWidgetFocus`
  (params (Key :type "Key Structure" :default "None"))
  (`WidgetInteractionComponent.PressAndReleaseKey` (`self.WidgetInteractionComp`) Key))

(event `OnWidgetClosed_Event_0`
  ;[1 1 1] Open Pause Menu
  (`Widget.SetVisibility` (`self.PauseMenu`) "Collapsed" :!label _label)
  (set `self.bShowMouseCursor` false)
  (`WidgetBlueprintLibrary.SetInputMode_GameOnly` self))

(event `SetInputMode3DWidget`
  (params (InWidgetToFocus :type "Widget Object Reference"))
  (set `self.FocuseWidget` InWidgetToFocus)
  (set `self.bShowMouseCursor` true)
  (`WidgetBlueprintLibrary.SetInputMode_GameAndUIEx` self InWidgetToFocus "LockInFullscreen")
  (set `WidgetInteractionComponent.InteractionSource` "Mouse" (`self.WidgetInteractionComp`))
  (`self.DisableInput` (`self.K2_GetPawn`) self))

(event `InputAction|OpenMenu`
  (params (Key :type "Key Structure"))
  ;[1 1 1] Open Pause Menu
  (:`Pressed`
    (bind _pausemenu (`self.PauseMenu`)
      (:`then`
        (if (`Widget.IsVisible` _pausemenu)
          (goto _label)
          (else
            (`Widget.SetVisibility` (`self.PauseMenu`) "Visible"))))
      (:`else`
        (bind _returnvalue (`|CreateWidget` "/Game/Widgets/W_MainMenu.W_MainMenu_C"))
        (bind _output_get (set `self.PauseMenu` _returnvalue))
        (`UserWidget.AddToViewport` _output_get 0)
        (add `/Game/Widgets/W_MainMenu.OnWidgetClosed` _output_get (delegate `OnWidgetClosed_Event_0`))))
    (set `self.bShowMouseCursor` true)
    (`WidgetBlueprintLibrary.SetInputMode_UIOnlyEx` self null)))

(event `SetInputModeGame`
  (set `self.bShowMouseCursor` false)
  (set `WidgetInteractionComponent.InteractionSource` "CenterScreen" (`self.WidgetInteractionComp`))
  (`WidgetBlueprintLibrary.SetInputMode_GameOnly` self)
  (`self.EnableInput` (`self.K2_GetPawn`) self)
  (set `self.FocuseWidget` null))

(event `InputAction|OpenTextChat`
  (params (Key :type "Key Structure"))
  (bind _w_chatwindow (`/Game/PlayerCharacter/Hud/W_Hud.W_ChatWindow` (`self.Hud`)))
  ;[1 1 1] Open Chat
  (:`Pressed`
    (`WidgetBlueprintLibrary.SetInputMode_UIOnlyEx` self _w_chatwindow)
    (`/Game/PlayerCharacter/Hud/W_ChatWindow.SetFocusToTextInput` _w_chatwindow)
    (set `self.bShowMouseCursor` true)))

(fn `UserConstructionScript`)