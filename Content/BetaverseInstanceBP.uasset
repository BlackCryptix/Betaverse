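; Game instance Blueprint for Betaverse that applies saved audio volumes at startup and manages a global loading screen.
; On Init, after a short delay, it activates the MixGlobal sound mix and applies saved Master, SFX, Music and Voice levels through SetVolume.
; SetVolume loads settings if missing, sets a clamped sound class override on the mix and saves the value back to Settings.
; The loading screen widget is created once, cached, then added to or removed from the viewport on demand.
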(event `self.ReceiveInit`
  (bind (_soundsettings_master _soundsettings_sfx _soundsettings_music _soundsettings_voice) (break `SoundSettings` (`SettingsSaveGame.SoundSettings` (`self.Settings`))))
  ;[1 1 1] Init
  (`parent.ReceiveInit`)
  (`KismetSystemLibrary.Delay` 0.2)
  ;;[1 1 1] Set sound mixes
  (`GameplayStatics.SetBaseSoundMix` "/Game/AudioSettings/MixGlobal.MixGlobal")
  (`GameplayStatics.PushSoundMixModifier` "/Game/AudioSettings/MixGlobal.MixGlobal")
  ;;[1 1 1] Load and set volume levels
  (`|ExecutionSequence`
    (:`then_0`
      (`self.SetVolume` "NewEnumerator0" _soundsettings_master))
    (:`then_1`
      (`self.SetVolume` "NewEnumerator2" _soundsettings_sfx))
    (:`then_2`
      (`self.SetVolume` "NewEnumerator1" _soundsettings_music))
    (:`then_3`
      (`self.SetVolume` "NewEnumerator3" _soundsettings_voice))))

(event `ShowLoadingScreen`
  ;[1 1 1] LaodingScreen
  (`self.LoadingScreen`
    (:`then`
      _)
    (:`else`
      (bind _returnvalue (`|CreateWidget` "/Game/Widgets/W_LoadingScreen.W_LoadingScreen_C"))
      (set `self.LoadingScreen` _returnvalue)))
  (`UserWidget.AddToViewport` (`self.LoadingScreen`) 10))

(event `RemoveLoadingScreen`
  ;[1 1 1] LaodingScreen
  (bind _loadingscreen (`self.LoadingScreen`)
    (:`then`
      (`Widget.RemoveFromParent` _loadingscreen))
    (:`else`)))

(fn `SetVolume`
  (params (SoundChannel :type "/Game/AudioSettings/E_SoundChannel Enum" :default "NewEnumerator0") (Value :type "Float (double-precision)"))
  (bind _returnvalue (`KismetMathLibrary.FClamp` Value))
  (`/Engine/EditorBlueprintResources/StandardMacros.IsValid` (`self.Settings`)
    (:`Is Valid`
      _)
    (:`Is Not Valid`
      (`self.LoadGameSettings`)))
  (switch `/Game/AudioSettings/E_SoundChannel` SoundChannel
    (:`NewEnumerator0`
      (`GameplayStatics.SetSoundMixClassOverride` "/Game/AudioSettings/MixGlobal.MixGlobal" "/Game/AudioSettings/Master.Master" _returnvalue)
      (`SettingsSaveGame.SaveMasterVolume` (`self.Settings`) _returnvalue))
    (:`NewEnumerator1`
      (`GameplayStatics.SetSoundMixClassOverride` "/Game/AudioSettings/MixGlobal.MixGlobal" "/Game/AudioSettings/Music.Music" _returnvalue)
      (`SettingsSaveGame.SaveMusicVolume` (`self.Settings`) _returnvalue))
    (:`NewEnumerator2`
      (`GameplayStatics.SetSoundMixClassOverride` "/Game/AudioSettings/MixGlobal.MixGlobal" "/Game/AudioSettings/SFX.SFX" _returnvalue)
      (`SettingsSaveGame.SaveSFXVolume` (`self.Settings`) _returnvalue))
    (:`NewEnumerator3`
      (`GameplayStatics.SetSoundMixClassOverride` "/Game/AudioSettings/MixGlobal.MixGlobal" "/Game/AudioSettings/Voice.Voice" _returnvalue)
      (`SettingsSaveGame.SaveVoiceVolume` (`self.Settings`) _returnvalue))))